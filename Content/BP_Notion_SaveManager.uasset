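; BP_Notion_SaveManager manages saving and loading of the Notion property and paint save data.
; Init loads both BP_Notion_SaveData and BP_Notion_PaintSaveData from their own fixed slots, creating a fresh object when a slot load fails the cast.
; Separate save events write each held object back to its slot, so property and paint data persist independently.
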(event `Init`
  (`self.LoadPropertyData`)
  (`self.LoadPaintData`))

(event `SavePaintData`
  (`GameplayStatics.SaveGameToSlot` (`self.PaintSaveData`) "NotionPaintData"))

(event `LoadPaintData`
  (bind _returnvalue (`GameplayStatics.LoadGameFromSlot` "NotionPaintData"))
  (bind _asbp_notion_paint_save_data (cast `/NotionUnreal/BP_Notion_PaintSaveData` _returnvalue)
    (:`then`
      (set `self.PaintSaveData` _asbp_notion_paint_save_data))
    (:`CastFailed`
      (bind _returnvalue_2 (`GameplayStatics.CreateSaveGameObject` "/NotionUnreal/BP_Notion_PaintSaveData.BP_Notion_PaintSaveData_C"))
      (set `self.PaintSaveData` _returnvalue_2))))

(event `SavePropertyData`
  (`GameplayStatics.SaveGameToSlot` (`self.PropertySaveData`) "NotionPropertyData"))

(event `LoadPropertyData`
  (bind _returnvalue (`GameplayStatics.LoadGameFromSlot` "NotionPropertyData"))
  (bind _asbp_notion_save_data (cast `/NotionUnreal/BP_Notion_SaveData` _returnvalue)
    (:`then`
      (set `self.PropertySaveData` _asbp_notion_save_data))
    (:`CastFailed`
      (bind _returnvalue_2 (`GameplayStatics.CreateSaveGameObject` "/NotionUnreal/BP_Notion_SaveData.BP_Notion_SaveData_C"))
      (set `self.PropertySaveData` _returnvalue_2))))